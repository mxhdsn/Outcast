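; Pumpkin enemy actor that jumpscares the first-person character on contact and sends the game back to the main menu.
; From BeginPlay, a self-calling Laugh event replays a laugh sound after each delay.
; Box overlap shows the character's pumpkin and unpauses its JumpScare, using IsbeingScared as a guard, then after a pause resets both state and playback and opens MainMenu.
; A look-at-player timeline is disconnected and never runs.
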(event OnComponentBeginOverlap(Box)
  (params (OverlappedComponent :type Primitive%20Component%20Object%20Reference) (OtherActor :type Actor%20Object%20Reference) (OtherComp :type Primitive%20Component%20Object%20Reference) (OtherBodyIndex :type Integer) (bFromSweep :type Boolean) (SweepResult :type Hit%20Result%20Structure%20%28by%20ref%29))
  (bind _asbp_first_person_character (Utilities|Casting|CastToBP_FirstPersonCharacter OtherActor))
  (if (not (Variables|/Game/FirstPerson/Blueprints/BP_FirstPersonCharacter.BP_FirstPersonCharacter_C|GetisbeingScared _asbp_first_person_character))
    (Rendering|SetVisibility (Variables|/Game/FirstPerson/Blueprints/BP_FirstPersonCharacter.BP_FirstPersonCharacter_C|GetHalloweenPumpkin _asbp_first_person_character) true false)
    (Variables|/Game/FirstPerson/Blueprints/BP_FirstPersonCharacter.BP_FirstPersonCharacter_C|SetisbeingScared _asbp_first_person_character true)
    (Class|AudioComponent|SetPaused (Variables|/Game/FirstPerson/Blueprints/BP_FirstPersonCharacter.BP_FirstPersonCharacter_C|GetJumpScare _asbp_first_person_character) false)
    (Utilities|FlowControl|Delay 2.0)
    (Class|AudioComponent|SetPaused (Variables|/Game/FirstPerson/Blueprints/BP_FirstPersonCharacter.BP_FirstPersonCharacter_C|GetJumpScare _asbp_first_person_character) true)
    (Variables|/Game/FirstPerson/Blueprints/BP_FirstPersonCharacter.BP_FirstPersonCharacter_C|SetisbeingScared _asbp_first_person_character false)
    (Game|OpenLevel(byName) "MainMenu")))

(event Custom|Laugh
  (Utilities|FlowControl|Delay 1e+01)
  (Audio|Components|Audio|Play (Variables|Default|GetHeheheha) 0.0)
  (CallFunction|Laugh))

(event EventBeginPlay
  (CallFunction|Laugh))

(fn ConstructionScript)