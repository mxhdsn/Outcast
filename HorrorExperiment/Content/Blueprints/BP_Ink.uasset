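; BP_Ink is a collectible ink pickup that registers with the first-person player character when collected.
; A timeline event callback checks whether player 0's BP_FirstPersonCharacter is interacting.
; If so, it sets the character's ink-collected flag, increments its collected item count and destroys itself.
; The graph shows no proximity check or timeline start, and the construction script only calls the parent's.
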(event EventTimelineCheckEEventFunc
  (bind _asbp_first_person_character (Utilities|Casting|CastToBP_FirstPersonCharacter (Game|GetPlayerCharacter 0)))
  (if (Variables|/Game/FirstPerson/Blueprints/BP_FirstPersonCharacter.BP_FirstPersonCharacter_C|GetisInteracting _asbp_first_person_character)
    (Variables|/Game/FirstPerson/Blueprints/BP_FirstPersonCharacter.BP_FirstPersonCharacter_C|SethasCollectedInk _asbp_first_person_character true)
    (bind _result (Math|Float|IncrementFloat (Variables|/Game/FirstPerson/Blueprints/BP_FirstPersonCharacter.BP_FirstPersonCharacter_C|GetitemsCollected _asbp_first_person_character))
      (:%20%20
        (Variables|/Game/FirstPerson/Blueprints/BP_FirstPersonCharacter.BP_FirstPersonCharacter_C|SetitemsCollected _asbp_first_person_character _result)
        (Actor|DestroyActor)))))

(fn ConstructionScript
  (|CallParentFunction))