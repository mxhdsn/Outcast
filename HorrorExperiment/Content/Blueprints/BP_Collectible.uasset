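; BP_Collectible is a spinning pickup that shows the first-person character's interact prompt while the player is inside its Box.
; Overlap starts a Timeline whose Check E event tests IsInteracting and hides the prompt; leaving hides it and stops the Timeline.
; A separate SpinTimeline drives delta-time-scaled yaw rotation from BeginPlay.
; Interacting only hides the prompt, with no collection or destroy logic here.
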(event OnComponentBeginOverlap(Box)
  (params (OverlappedComponent :type Primitive%20Component%20Object%20Reference) (OtherActor :type Actor%20Object%20Reference) (OtherComp :type Primitive%20Component%20Object%20Reference) (OtherBodyIndex :type Integer) (bFromSweep :type Boolean) (SweepResult :type Hit%20Result%20Structure%20%28by%20ref%29))
  (bind _asbp_first_person_character (Utilities|Casting|CastToBP_FirstPersonCharacter OtherActor)
    (:then
      (Variables|/Game/FirstPerson/Blueprints/BP_FirstPersonCharacter.BP_FirstPersonCharacter_C|SetInteractVisible _asbp_first_person_character true)
      (Timeline|Timeline PlayFromStart
        (:CheckE
          (if (Variables|/Game/FirstPerson/Blueprints/BP_FirstPersonCharacter.BP_FirstPersonCharacter_C|GetisInteracting _asbp_first_person_character)
            (Variables|/Game/FirstPerson/Blueprints/BP_FirstPersonCharacter.BP_FirstPersonCharacter_C|SetInteractVisible _asbp_first_person_character false)))))
    (:CastFailed
      (Development|PrintString "Error, something other than player collided with collectible" true true "(R=1.000000,G=0.000000,B=0.000000,A=1.000000)"))))

(event OnComponentEndOverlap(Box)
  (params (OverlappedComponent :type Primitive%20Component%20Object%20Reference) (OtherActor :type Actor%20Object%20Reference) (OtherComp :type Primitive%20Component%20Object%20Reference) (OtherBodyIndex :type Integer))
  (bind _asbp_first_person_character (Utilities|Casting|CastToBP_FirstPersonCharacter OtherActor))
  (Variables|/Game/FirstPerson/Blueprints/BP_FirstPersonCharacter.BP_FirstPersonCharacter_C|SetInteractVisible _asbp_first_person_character false)
  (Timeline|Timeline Stop
    (:CheckE
      (if (Variables|/Game/FirstPerson/Blueprints/BP_FirstPersonCharacter.BP_FirstPersonCharacter_C|GetisInteracting (stale OnComponentBeginOverlap(Box) _asbp_first_person_character))
        (Variables|/Game/FirstPerson/Blueprints/BP_FirstPersonCharacter.BP_FirstPersonCharacter_C|SetInteractVisible (stale OnComponentBeginOverlap(Box) _asbp_first_person_character) false)))))

(event Custom|Spin
  (bind _newtrack_0 (Timeline|Spin%20Timeline PlayFromStart)
    (:Update
      (Transformation|AddActorLocalRotation (Math|Rotator|MakeRotator 0.0 0.0 (* _newtrack_0 (Utilities|Time|GetWorldDeltaSeconds))) false false))))

(event EventBeginPlay
  (CallFunction|Spin))

(fn ConstructionScript)